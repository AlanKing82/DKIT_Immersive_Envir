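; Pedestal play button Blueprint that starts a referenced Animation's playback when interacted with and flashes when focused.
; The construction script gives the button a dynamic blue material, whose Brightness OnFocus raises for one second.
; OnInteract, if Animation is valid, calls PlayAnimation and runs a timeline into UpdateButton.
; UpdateButton ignores the timeline value, setting the button at a fixed one-unit Z offset from its BeginPlay location.
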(event EventOnFocus
  (bind _buttonmatinstance (Variables|Default|GetButtonMatInstance))
  (Variables|Default|SetHighLightOn true)
  (if (Variables|Default|GetHighLightOn)
    (Rendering|Material|SetScalarParameterValue _buttonmatinstance "Brightness" 1e+01 :!class /Script/Engine.MaterialInstanceDynamic)
    (Variables|Default|SetHighLightOn false)
    (Utilities|FlowControl|Delay 1.0)
    (Rendering|Material|SetScalarParameterValue _buttonmatinstance "Brightness" 0.0 :!class /Script/Engine.MaterialInstanceDynamic)
    (Variables|Default|SetHighLightOn true)))

(event EventBeginPlay
  (Variables|Default|SetInitialButtonLoc (Transformation|GetWorldLocation (Variables|Default|GetButton))))

(event EventOnInteract
  (bind _animation (Variables|Default|GetAnimation))
  (Utilities|IsValid _animation
    (:Is%20Valid
      (Default|PlayAnimation _animation)
      (bind _buttonpress (Timeline|Timeline_0 Play)
        (:Update
          (CallFunction|UpdateButton _buttonpress))))))

(fn ConstructionScript
  (bind _returnvalue (Rendering|Material|CreateDynamicMaterialInstance "/Game/ExampleContent/Blueprints/Materials/M_Blue_Shiny_Inst.M_Blue_Shiny_Inst" "None" :!class /Script/Engine.KismetMaterialLibrary))
  (bind _output_get (Variables|Default|SetButtonMatInstance _returnvalue))
  (Rendering|Material|SetMaterial (Variables|Default|GetButton) 0 _output_get))

(fn UpdateButton
  (params (ButtonElevation :type Float%20%28single-precision%29))
  (bind _initialbuttonloc (Variables|Default|GetInitialButtonLoc))
  (bind (_x _y _z) (Math|Vector|BreakVector _initialbuttonloc))
  ;[1 1 1] Set button location
  (Transformation|SetWorldLocation (Variables|Default|GetButton) (Math|Vector|MakeVector _x _y (+ _z 1.0)) false false))