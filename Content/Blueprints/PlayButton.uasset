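; PlayButton is a Blueprint for a play button in the world that glows on focus and reacts to presses.
; Construction creates a dynamic material instance, whose Brightness parameter the focus and blur events raise or clear.
; PressPlay runs a timeline that calls UpdateButton each update to set the button's location from its BeginPlay position.
; UpdateButton ignores the timeline's elevation value and applies a fixed Z offset.
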(event Custom|ButtonFocused
  (Rendering|Material|SetScalarParameterValue (Variables|Default|GetButtonMatInstance) "Brightness" 1e+01 :!class /Script/Engine.MaterialInstanceDynamic))

(event Custom|ButtonBlurred
  (Rendering|Material|SetScalarParameterValue (Variables|Default|GetButtonMatInstance) "Brightness" 0.0 :!class /Script/Engine.MaterialInstanceDynamic))

(event Custom|PressPlay
  (bind _buttonpress (Timeline|Timeline_0 Play)
    (:Update
      (CallFunction|UpdateButton _buttonpress))))

(event EventBeginPlay
  (Variables|Default|SetInitialButtonLoc (Transformation|GetWorldLocation (Variables|Default|GetButton))))

(fn ConstructionScript
  (bind _returnvalue (Rendering|Material|CreateDynamicMaterialInstance "/Game/ExampleContent/Blueprints/Materials/M_Blue_Shiny_Inst.M_Blue_Shiny_Inst" "None" :!class /Script/Engine.KismetMaterialLibrary))
  (bind _output_get (Variables|Default|SetButtonMatInstance _returnvalue))
  (Rendering|Material|SetMaterial (Variables|Default|GetButton) 0 _output_get))

(fn UpdateButton
  (params (ButtonElevation :type Float%20%28single-precision%29))
  (bind _initialbuttonloc (Variables|Default|GetInitialButtonLoc))
  (bind (_x _y _z) (Math|Vector|BreakVector _initialbuttonloc))
  ;[1 1 1] Set button location
  (Transformation|SetWorldLocation (Variables|Default|GetButton) (Math|Vector|MakeVector _x _y (+ _z 1.0)) false false))