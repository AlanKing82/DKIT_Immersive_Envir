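; VR player controller that provides gaze-aimed teleport and glide movement for the player pawn.
; Each tick it traces from the camera and projects the hit onto the navmesh, moving a spawned VRPreviewBP marker there or hiding its sphere.
; Teleport repeats that check and jumps the pawn to the projected point, raised slightly.
; Glide uses a timeline to lerp the pawn toward the traced impact point in XY only, without a navmesh check.
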(event EventTick
  (params (DeltaSeconds :type Float%20%28single-precision%29))
  (bind _returnvalue (Game|GetPlayerCameraManager 0))
  (bind _returnvalue_2 (Transformation|GetActorLocation _returnvalue))
  (bind _outhit (Collision|LineTraceByChannel _returnvalue_2 (+ _returnvalue_2 (* (Transformation|GetActorForwardVector _returnvalue) (Variables|Default|GetTeleportDistance))) "TraceTypeQuery1" false 0 "None"))
  (Variables|Default|SetViewObject (.HitActor (Collision|BreakHitResult _outhit)))
  (bind _output_get (Variables|Default|SetCanTeleport (.ReturnValue (AI|Navigation|ProjectPointtoNavigation (.Location (Collision|BreakHitResult _outhit)) 0 0 "0, 0, 0"))))
  (if _output_get
    (Rendering|SetVisibility (Variables|/Game/Blueprints/VRPreviewBP.VRPreviewBP_C|GetVRPreviewSphere (stale EventBeginPlay _output_get)) true false)
    (Transformation|SetActorLocation (stale EventBeginPlay _returnvalue) (.ProjectedLocation (AI|Navigation|ProjectPointtoNavigation (.Location (Collision|BreakHitResult _outhit)) 0 0 "0, 0, 0")) false false)
    (else
      (Rendering|SetVisibility (Variables|/Game/Blueprints/VRPreviewBP.VRPreviewBP_C|GetVRPreviewSphere (stale EventBeginPlay _output_get)) false false))))

(event EventBeginPlay
  (Variables|Default|SetPlayerRef (Game|Player|GetPlayerPawn 0))
  (bind _returnvalue (Game|SpawnActorfromClass "/Game/Blueprints/VRPreviewBP.VRPreviewBP_C" (Math|Conversions|ToTransform(Vector) (.Location (Collision|BreakHitResult (stale EventTick _outhit)))) "Undefined" 0 0))
  (bind _output_get (Variables|Default|SetVRPreview _returnvalue)))

(event Input|ActionEvents|InputActionGlide
  (params (Key :type Key%20Structure :default "None"))
  (bind _returnvalue (Game|GetPlayerCameraManager 0))
  (bind _playerref (Variables|Default|GetPlayerRef))
  (bind _returnvalue_2 (Transformation|GetActorLocation _returnvalue))
  (:Pressed
    (bind _outhit (Collision|LineTraceByChannel _returnvalue_2 (+ _returnvalue_2 (* (Transformation|GetActorForwardVector _returnvalue) (Variables|Default|GetGlideDistance))) "TraceTypeQuery1" false 0 "None"))
    (bind _output_get (Variables|Default|SetEndTrace (.ImpactPoint (Collision|BreakHitResult _outhit))))
    (bind _output_get_2 (Variables|Default|SetStartTrace (Transformation|GetActorLocation (Game|Player|GetPlayerPawn 0))))
    (Components|Timeline|SetPlayRate (Variables|Default|GetGlideCurve) (/ 1.0 (Variables|Default|GetRateOfGlide)))
    (bind _glidefloat (Timeline|GlideCurve PlayFromStart)
      (:Update
        (Transformation|SetActorLocation _playerref (Math|Vector|MakeVector (.x (Math|Vector|Lerp(Vector) _output_get_2 _output_get _glidefloat)) (.y (Math|Vector|Lerp(Vector) _output_get_2 _output_get _glidefloat)) (.z (Transformation|GetActorLocation _playerref))) false false)))))

(event Input|ActionEvents|InputActionTeleport
  (params (Key :type Key%20Structure :default "None"))
  (bind _returnvalue (Game|GetPlayerCameraManager 0))
  (bind _returnvalue_2 (Transformation|GetActorLocation _returnvalue))
  (:Pressed
    (bind _outhit (Collision|LineTraceByChannel _returnvalue_2 (+ _returnvalue_2 (* (Transformation|GetActorForwardVector _returnvalue) (Variables|Default|GetTeleportDistance))) "TraceTypeQuery1" false 0 "None"))
    (bind _output_get (Variables|Default|SetCanTeleport (.ReturnValue (AI|Navigation|ProjectPointtoNavigation (.Location (Collision|BreakHitResult _outhit)) 0 0 "0, 0, 0"))))
    (if _output_get
      (Transformation|SetActorLocation (Variables|Default|GetPlayerRef) (+ (.ProjectedLocation (AI|Navigation|ProjectPointtoNavigation (.Location (Collision|BreakHitResult _outhit)) 0 0 "0, 0, 0")) "0, 0,90.000000") false false))))

(fn ConstructionScript)