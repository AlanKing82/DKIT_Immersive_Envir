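; PodBP is a pad that the VR player can jump to by looking at it and activating.
; On BeginPlay it caches the VRPawnBP and binds JumpToPad to its activate dispatcher, which moves the player to the pad's location if the pawn's OtherViewObjectRef is this pod.
; Tick polls that same reference to show the Indicator only while this pod is the viewed object.
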(event Custom|JumpToPad
  (bind _self self)
  (Development|PrintString "Hello")
  (if (== (Variables|/Game/Blueprints/VRPawnBP.VRPawnBP_C|GetOtherViewObjectRef (Variables|Default|Getplayer)) _self)
    (Transformation|SetActorLocation (Variables|Default|Getplayer) (Transformation|GetActorLocation _self) false false)))

(event EventTick
  (params (DeltaSeconds :type Float%20%28single-precision%29))
  (bind _indicator (Variables|Default|GetIndicator))
  ;[1 1 1] Indicator visibility
  (if (== (Variables|/Game/Blueprints/VRPawnBP.VRPawnBP_C|GetOtherViewObjectRef (Variables|Default|Getplayer)) self)
    (Rendering|SetVisibility _indicator true false)
    (else
      (Rendering|SetVisibility _indicator false false))))

(event EventBeginPlay
  (bind _asvrpawn_bp (Utilities|Casting|CastToVRPawnBP (Game|Player|GetPlayerPawn 0)))
  (EventDispatchers|BindEventtoActivateDispatch _asvrpawn_bp (delegate Custom|JumpToPad))
  (Variables|Default|Setplayer _asvrpawn_bp))

(fn ConstructionScript)