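; Oculus Go controller Blueprint that highlights individual buttons on its controller model.
; Start and Stop events for the trigger, Back, Home and trackpad swap that part's material slot between the highlight and default materials.
; On each Start, UpdateHighlightMaterial creates a dynamic material instance on the slot and applies the configurable highlight color and power.
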(event Custom|Trackpad_Highlight_Start
  ;[0.0643 0.3193 1] Handle Button Highlighting
  (Rendering|Material|SetMaterial (Variables|Default|GetControllerModel) 4 "/Game/OculusGoController/Materials/M_OculusGoController_Highlight.M_OculusGoController_Highlight")
  (CallFunction|UpdateHighlightMaterial 4))

(event Custom|Button_Back_Highlight_Stop
  ;[0.0643 0.3193 1] Handle Button Highlighting
  (Rendering|Material|SetMaterial (Variables|Default|GetControllerModel) 2 "/Game/OculusGoController/Materials/M_OculusGoController.M_OculusGoController"))

(event Custom|Button_Back_Highlight_Start
  ;[0.0643 0.3193 1] Handle Button Highlighting
  (Rendering|Material|SetMaterial (Variables|Default|GetControllerModel) 2 "/Game/OculusGoController/Materials/M_OculusGoController_Highlight.M_OculusGoController_Highlight")
  (CallFunction|UpdateHighlightMaterial 2))

(event Custom|Trackpad_Highlight_Stop
  ;[0.0643 0.3193 1] Handle Button Highlighting
  (Rendering|Material|SetMaterial (Variables|Default|GetControllerModel) 4 "/Game/OculusGoController/Materials/M_OculusGoController.M_OculusGoController"))

(event Custom|Button_Home_Highlight_Stop
  ;[0.0643 0.3193 1] Handle Button Highlighting
  (Rendering|Material|SetMaterial (Variables|Default|GetControllerModel) 3 "/Game/OculusGoController/Materials/M_OculusGoController.M_OculusGoController"))

(event Custom|Button_Trigger_Highlight_Stop
  ;[0.0643 0.3193 1] Handle Button Highlighting
  (Rendering|Material|SetMaterial (Variables|Default|GetControllerModel) 1 "/Game/OculusGoController/Materials/M_OculusGoController.M_OculusGoController"))

(event Custom|Button_Home_Highlight_Start
  ;[0.0643 0.3193 1] Handle Button Highlighting
  (Rendering|Material|SetMaterial (Variables|Default|GetControllerModel) 3 "/Game/OculusGoController/Materials/M_OculusGoController_Highlight.M_OculusGoController_Highlight")
  (CallFunction|UpdateHighlightMaterial 3))

(event Custom|Button_Trigger_Highlight_Start
  ;[0.0643 0.3193 1] Handle Button Highlighting
  (Rendering|Material|SetMaterial (Variables|Default|GetControllerModel) 1 "/Game/OculusGoController/Materials/M_OculusGoController_Highlight.M_OculusGoController_Highlight")
  (CallFunction|UpdateHighlightMaterial 1))

(fn ConstructionScript)

(fn UpdateHighlightMaterial
  (params (MaterialID :type Integer))
  (bind _controllermodel (Variables|Default|GetControllerModel))
  (bind _returnvalue (Rendering|Material|CreateDynamicMaterialInstance _controllermodel MaterialID (Rendering|Material|GetMaterial _controllermodel MaterialID) :!class /Script/Engine.PrimitiveComponent))
  (Rendering|Material|SetVectorParameterValue _returnvalue "Color" (Variables|Settings|GetButtonHighlightColor) :!class /Script/Engine.MaterialInstanceDynamic)
  (Rendering|Material|SetScalarParameterValue _returnvalue "Power" (Variables|Settings|GetButtonHighlightPower) :!class /Script/Engine.MaterialInstanceDynamic))